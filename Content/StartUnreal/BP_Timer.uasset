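; BP_Timer is a toggleable stopwatch that prints elapsed minutes and seconds with Korean unit labels.
; BeginPlay binds to the Pawn's ClickY event dispatcher, with an auto-generated function that flips IsPlay to start or pause timing.
; While playing, Tick calls CountDown, which despite its name counts up by Speed-scaled delta time.
; CountDown caches the last formatted string so it prints only when the displayed time changes.
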(event EventBeginPlay
  (EventDispatchers|BindEventtoEventDispatcherClickY (Variables|Default|GetPawn) (EventDispatchers|CreateEvent :!event BPTimerAutoGenFunc)))

(event EventTick
  (params (DeltaSeconds :type Float%20%28single-precision%29))
  (if (Variables|Default|GetIsPlay)
    (CallFunction|CountDown DeltaSeconds)))

(fn ConstructionScript)

(fn CountDown
  (params (DeltaSeconds :type Float%20%28single-precision%29))
  (bind _output_get (Variables|Default|SetTotalDeltaSeconds (+ (* DeltaSeconds (Variables|Default|GetSpeed)) (Variables|Default|GetTotalDeltaSeconds))))
  (if (not (Utilities|Enum|Equal(Enum) (Variables|Default|GetBeforeStr) (Utilities|String|Append (Utilities|String|ToString(Integer) (Math|Float|Floor (/ _output_get 6e+01))) "분" (Utilities|String|ToString(Integer) (Math|Float|Floor (Math|Float|%(Float) _output_get 6e+01))) "초")))
    (Development|PrintString (Utilities|String|Append (Utilities|String|ToString(Integer) (Math|Float|Floor (/ _output_get 6e+01))) "분" (Utilities|String|ToString(Integer) (Math|Float|Floor (Math|Float|%(Float) _output_get 6e+01))) "초"))
    (Variables|Default|SetBeforeStr (Utilities|String|Append (Utilities|String|ToString(Integer) (Math|Float|Floor (/ _output_get 6e+01))) "분" (Utilities|String|ToString(Integer) (Math|Float|Floor (Math|Float|%(Float) _output_get 6e+01))) "초"))))

(fn BPTimerAutoGenFunc
  (Variables|Default|SetIsPlay (not (Variables|Default|GetIsPlay))))