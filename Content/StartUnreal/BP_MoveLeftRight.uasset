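; Blueprint actor that moves its Sphere component back and forth along its relative X axis.
; Each Tick offsets the sphere by a step scaled by Speed and DeltaSeconds, with the IsRightMove flag selecting the branch.
; The flag flips when relative X passes fixed upper and lower bounds, producing a continuous ping-pong motion.
; A disconnected switch on NewVar0 never runs.
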(event EventTick
  (params (DeltaSeconds :type Float%20%28single-precision%29))
  (bind _sphere (Variables|Default|GetSphere))
  (bind _speed (Variables|Default|GetSpeed))
  (bind _returnvalue (* DeltaSeconds _speed))
  (if (Variables|Default|GetIsRightMove)
    (Transformation|AddRelativeLocation _sphere (Math|Vector|MakeVector _returnvalue 0.0 0.0) false false)
    (if (> (.x (Variables|/Script/Engine.SceneComponent|GetRelativeLocation _sphere)) 1e+02)
      (Variables|Default|SetIsRightMove false))
    (else
      (bind _result (Math|Float|NegateFloat _returnvalue)
        (:%20%20
          (Transformation|AddRelativeLocation _sphere (Math|Vector|MakeVector _result 0.0 0.0) false false)
          (if (<= (.x (Variables|/Script/Engine.SceneComponent|GetRelativeLocation _sphere)) 0.0)
            (Variables|Default|SetIsRightMove true)))))))

(fn ConstructionScript)