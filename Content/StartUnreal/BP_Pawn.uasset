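; BP_Pawn is a simple controllable pawn with basic movement, look input and debug prints on BeginPlay and Enter.
; Move axes offset the actor along its forward and right vectors at a fixed per-tick step, without sweep or delta-time scaling.
; Look axes feed controller rotation with names crossed: LookUp drives yaw and LookRight drives pitch.
; The Y key broadcasts the ClickY event dispatcher to any bound listeners.
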(event EventBeginPlay
  (Development|PrintString "BeginPlay"))

(event Input|ActionEvents|InputActionEnterInput
  (params (Key :type Key%20Structure :default "None"))
  (:Pressed
    (Development|PrintString "Enter 키 Pressed")))

(event Input|AxisEvents|InputAxisLookUp
  (params (AxisValue :type Float%20%28single-precision%29))
  (Pawn|Input|AddControllerYawInput AxisValue))

(event Input|AxisEvents|InputAxisLookRight
  (params (AxisValue :type Float%20%28single-precision%29))
  (Pawn|Input|AddControllerPitchInput AxisValue))

(event Input|AxisEvents|InputAxisMoveRight
  (params (AxisValue :type Float%20%28single-precision%29))
  (Transformation|AddActorWorldOffset (* (Transformation|GetActorRightVector) (* AxisValue 1e+01))))

(event Input|AxisEvents|InputAxisMoveForward
  (params (AxisValue :type Float%20%28single-precision%29))
  ;[0.3298 1 0.2087 1 20] 앞쪽으로 움직임
  (Transformation|AddActorWorldOffset (* (Transformation|GetActorForwardVector) (* AxisValue 1e+01))))

(event Input|KeyboardEvents|Y
  (params (Key :type Key%20Structure :default "None"))
  (:Pressed
    (Default|CallEventDispatcherClickY)))

(fn ConstructionScript)