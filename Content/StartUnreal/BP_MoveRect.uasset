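; BP_MoveRect moves its Sphere component around a square path in the local X-Z plane.
; Each Tick switches on MoveType and calls one of four direction functions, which offsets the Sphere's relative location by Speed scaled by delta time.
; Each function sets the next direction once the Sphere reaches its hardcoded bound, forming a looping state machine without clamping overshoot.
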(event EventTick
  (params (DeltaSeconds :type Float%20%28single-precision%29))
  (switch Utilities|FlowControl|Switch|SwitchonEnum_MoveType (Variables|Default|GetMoveType)
    (:NewEnumerator0
      (CallFunction|MoveRight DeltaSeconds))
    (:NewEnumerator1
      (CallFunction|MoveUp DeltaSeconds))
    (:NewEnumerator2
      (CallFunction|MoveLeft DeltaSeconds))
    (:NewEnumerator3
      (CallFunction|MoveDown DeltaSeconds))))

(fn ConstructionScript)

(fn MoveRight
  (params (DeltaSeconds :type Float%20%28single-precision%29))
  (bind _sphere (Variables|Default|GetSphere))
  (Transformation|AddRelativeLocation _sphere (Math|Vector|MakeVector (* DeltaSeconds (Variables|Default|GetSpeed)) 0.0 0.0) false false)
  (if (> (.x (Variables|/Script/Engine.SceneComponent|GetRelativeLocation _sphere)) 1e+02)
    (Variables|Default|SetMoveType "NewEnumerator1")))

(fn MoveLeft
  (params (DeltaSeconds :type Float%20%28single-precision%29))
  (bind _sphere (Variables|Default|GetSphere))
  (bind _result (Math|Float|NegateFloat (* DeltaSeconds (Variables|Default|GetSpeed)))
    (:%20%20
      (Transformation|AddRelativeLocation _sphere (Math|Vector|MakeVector _result 0.0 0.0) false false)
      (if (<= (.x (Variables|/Script/Engine.SceneComponent|GetRelativeLocation _sphere)) 0.0)
        (Variables|Default|SetMoveType "NewEnumerator3")))))

(fn MoveUp
  (params (DeltaSeconds :type Float%20%28single-precision%29))
  (bind _sphere (Variables|Default|GetSphere))
  (Transformation|AddRelativeLocation _sphere (Math|Vector|MakeVector 0.0 0.0 (* DeltaSeconds (Variables|Default|GetSpeed))) false false)
  (if (> (.z (Variables|/Script/Engine.SceneComponent|GetRelativeLocation _sphere)) 1e+02)
    (Variables|Default|SetMoveType "NewEnumerator2")))

(fn MoveDown
  (params (DeltaSeconds :type Float%20%28single-precision%29))
  (bind _sphere (Variables|Default|GetSphere))
  (bind _result (Math|Float|NegateFloat (* DeltaSeconds (Variables|Default|GetSpeed)))
    (:%20%20
      (Transformation|AddRelativeLocation _sphere (Math|Vector|MakeVector 0.0 0.0 _result) false false)
      (if (<= (.z (Variables|/Script/Engine.SceneComponent|GetRelativeLocation _sphere)) 0.0)
        (Variables|Default|SetMoveType "NewEnumerator0")))))